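; Fixed-camera variant that slides its spring arm along a spline to follow the player, ticking only while the camera's overlap is active.
; Each tick, the arm eases toward the spline point and rotation nearest the player, offset forward by an amount chosen from whether the player faces away from the camera.
; The cine camera can optionally turn toward the player on yaw and/or pitch.
; At construction, the arm snaps to a normalized CameraPoint along the spline.
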(event EventBeginPlay
  (|CallParentFunction) ; This node is disabled and will not be called.\nDrag off pins to build functionality.
)

(event EventTick
  (params (DeltaSeconds :type Float%20%28single-precision%29))
  (bind _returnvalue (Game|Player|GetPlayerPawn 0))
  (bind _returnvalue_2 (Game|Player|GetPlayerPawn 0))
  (bind _cinecamera (Variables|Default|GetCineCamera))
  (bind _cinecamera_2 (Variables|Default|GetCineCamera))
  (bind _returnvalue_3 (Transformation|GetWorldLocation _cinecamera_2))
  (bind _returnvalue_4 (Transformation|GetActorLocation _returnvalue_2))
  (bind _returnvalue_5 (Transformation|GetWorldRotation _cinecamera))
  (bind _returnvalue_6 (Math|Rotator|FindLookatRotation _returnvalue_3 _returnvalue_4))
  (Variables|Default|SetDelta%20Secondes DeltaSeconds)
  (CallFunction|SetPlayerCollisionOffSet)
  (Transformation|SetWorldLocation (Variables|Default|GetSpringArm) (Math|Interpolation|VInterpTo (Transformation|GetWorldLocation (Variables|Default|GetSpringArm)) (Spline|FindLocationClosesttoWorldLocation (Variables|Default|GetSpline) (+ (Transformation|GetActorLocation _returnvalue) (* (Transformation|GetActorForwardVector _returnvalue) (Variables|Default|GetPlayerCollisionOffSet))) "World") (Variables|Default|GetDelta%20Secondes) (Variables|Default|GetInterp%20Speed)) false false)
  (Transformation|SetWorldRotation (Variables|Default|GetSpringArm) (Math|Interpolation|RInterpTo (Transformation|GetWorldRotation (Variables|Default|GetSpringArm)) (Class|SplineComponent|FindRotationClosesttoWorldLocation (Variables|Default|GetSpline) (Transformation|GetWorldLocation (Variables|Default|GetSpringArm)) "World") (Variables|Default|GetDelta%20Secondes) (Variables|Default|GetInterp%20Speed)) false false)
  (if (or (Variables|Default|GetHorizontalPlayerFollow) (Variables|Default|GetVerticalPlayerFollow))
    (Transformation|SetWorldRotation (Variables|Default|GetCineCamera) (Math|Interpolation|RInterpTo (Transformation|GetWorldRotation (Variables|Default|GetCineCamera)) (Math|Rotator|MakeRotator (.roll _returnvalue_5) (Math|Float|SelectFloat (.pitch _returnvalue_6) (.pitch _returnvalue_5) (Variables|Default|GetVerticalPlayerFollow)) (Math|Float|SelectFloat (.yaw _returnvalue_6) (.yaw _returnvalue_5) (Variables|Default|GetHorizontalPlayerFollow))) (Variables|Default|GetDelta%20Secondes) (Variables|Default|GetInterp%20Speed)) false false)))

(fn ConstructionScript
  (|CallParentFunction)
  (CallFunction|SnaptoSpline))

(fn SnaptoSpline
  (bind _spline (Variables|Default|GetSpline))
  (bind _camerapoint (Variables|Default|GetCameraPoint))
  (bind _returnvalue (Spline|GetSplineLength _spline))
  (bind _returnvalue_2 (Math|Float|Lerp 0.0 _returnvalue _camerapoint))
  (Transformation|SetWorldTransform (Variables|Default|GetSpringArm) (Math|Transform|MakeTransform (Spline|GetLocationatDistanceAlongSpline (Variables|Default|GetSpline) _returnvalue_2 "World") (Spline|GetRotationatDistanceAlongSpline (Variables|Default|GetSpline) _returnvalue_2 "World") "1.000000,1.000000,1.000000") false false))

(fn OnFixedCameraOverlap
  (|CallParentFunction)
  (Actor|Tick|SetActorTickEnabled true))

(fn OnFixedCameraEndOverlap
  (|CallParentFunction)
  (Actor|Tick|SetActorTickEnabled false))

(fn SetPlayerCollisionOffSet
  (Variables|Default|SetPlayerCollisionOffSet (select (> (Math|Vector|DotProduct (Math|Vector|GetForwardVector (Variables|Default|GetCineCamera)) (Transformation|GetActorForwardVector (Game|Player|GetPlayerPawn 0))) 0.0) (Variables|Default|GetPlayerBackCollisionOffSetAmount) (Variables|Default|GetPlayerFrontCollisionOffSetAmount))))