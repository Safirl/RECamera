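; BP_FixedCamera is a placeable fixed camera that takes over the view when the player character enters its Box trigger.
; Box overlap, or a short delayed check after BeginPlay for a player already inside, blends the view target to this actor and optionally sets the CineCamera to track focus on the player pawn.
; Construction script sets spring arm length from a variable; the end-overlap handler is empty, so exiting restores nothing here.
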(event OnComponentBeginOverlap(Box)
  (params (OverlappedComponent :type Primitive%20Component%20Object%20Reference) (OtherActor :type Actor%20Object%20Reference) (OtherComp :type Primitive%20Component%20Object%20Reference) (OtherBodyIndex :type Integer) (bFromSweep :type Boolean) (SweepResult :type Hit%20Result%20Structure%20%28by%20ref%29))
  (if (== OtherActor (Game|GetPlayerCharacter 0))
    (CallFunction|OnFixedCameraOverlap)))

(event OnComponentEndOverlap(Box)
  (params (OverlappedComponent :type Primitive%20Component%20Object%20Reference) (OtherActor :type Actor%20Object%20Reference) (OtherComp :type Primitive%20Component%20Object%20Reference) (OtherBodyIndex :type Integer))
  (if (== OtherActor (Game|GetPlayerCharacter 0))
    (CallFunction|OnFixedCameraEndOverlap)))

(event Custom|CheckForPlayer
  (if (Collision|IsOverlappingActor (Variables|Default|GetBox) (Game|GetPlayerCharacter 0) :!class /Script/Engine.PrimitiveComponent)
    (CallFunction|OnFixedCameraOverlap)))

(event EventBeginPlay
  (Utilities|Time|SetTimerbyEvent (delegate Custom|CheckForPlayer) 0.1))

(fn ConstructionScript
  (Variables|/Script/Engine.SpringArmComponent|SetTargetArmLength (Variables|Default|GetSpringArm) (Variables|Default|GetSpringArmLenght)))

(fn OnFixedCameraOverlap
  (Game|Player|SetViewTargetwithBlend (Game|GetPlayerController 0) self (Variables|Default|GetBlend%20Time) (Variables|Default|GetBlend%20Func) 0.0 false)
  (if (Variables|Default|GetShouldFocusOnPlayer)
    (Variables|/Script/CinematicCamera.CineCameraComponent|SetFocusSettings (Variables|Default|GetCineCamera) (Utilities|Struct|MakeCameraFocusSettings "Tracking" 1e+05 (Utilities|Struct|MakeCameraTrackingFocusSettings (Utilities|ResolveSoftReference (Game|Player|GetPlayerPawn 0)) "0.000000,0.000000,0.000000" false) true))))

(fn OnFixedCameraEndOverlap)